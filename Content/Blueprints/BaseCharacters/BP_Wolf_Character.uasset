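; Wolf character Blueprint that performs a bite attack on the IA_Attack input.
; The input enables query collision on AttackCollider and, unless already attacking, sets IsAttacking, plays the bite montage and immediately disables the collider.
; Overlaps on the collider deal fixed damage to any BaseCharacter through OnAttackRecievedImplementation.
; IsAttacking is never cleared in this graph, and the IsRunning branch is empty.
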(event OnComponentBeginOverlap(AttackCollider)
  (params (OverlappedComponent :type Primitive%20Component%20Object%20Reference) (OtherActor :type Actor%20Object%20Reference) (OtherComp :type Primitive%20Component%20Object%20Reference) (OtherBodyIndex :type Integer) (bFromSweep :type Boolean) (SweepResult :type Hit%20Result%20Structure%20%28by%20ref%29))
  (bind _asbase_character (Utilities|Casting|CastToBaseCharacter OtherActor))
  (Class|BaseCharacter|OnAttackRecievedImplementation _asbase_character 2e+01 OverlappedComponent _asbase_character))

(event Input|EnhancedActionEvents|EnhancedInputActionIA_Attack
  (params (ActionValue :type Boolean) (ElapsedSeconds :type Float%20%28double-precision%29) (TriggeredSeconds :type Float%20%28double-precision%29) (InputAction :type Input%20Action%20Object%20Reference :default "/Game/inputs/IA_Attack.IA_Attack"))
  (Collision|SetCollisionEnabled (Variables|Default|GetAttackCollider) "QueryOnly")
  (if (Variables|Default|GetIsAttacking)
    (Development|PrintString "Still playing attack anim")
    (else
      (Variables|Default|SetIsAttacking true)
      (if (Variables|Default|GetisRunning)
        _
        (else
          _))
      (Animation|PlayAnimMontage "/Game/Animations/Animals/Wolf/MONT_Wolf_Bite.MONT_Wolf_Bite" 1.0 "None")
      (Collision|SetCollisionEnabled (Variables|Default|GetAttackCollider) "NoCollision"))))

(event EventBeginPlay)

(event Collision|EventActorBeginOverlap
  (params (OtherActor :type Actor%20Object%20Reference)))

(event EventTick
  (params (DeltaSeconds :type Float%20%28single-precision%29)))

(fn ConstructionScript)