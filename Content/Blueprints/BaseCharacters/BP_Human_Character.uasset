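; Human character Blueprint that handles menu input and scales walk speed to movement input strength.
; IA_Move maps the length of the last input vector to stepped MaxWalkSpeed values through a nested threshold chain, printing the length when it exceeds the top band.
; IA_Settings opens the options widget and IA_Menu calls ToggleMenu, both pausing the game with cursor and UI-only input.
; ToggleMenu only opens the menu; it has no close branch.
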(event Input|EnhancedActionEvents|EnhancedInputActionIA_Menu
  (params (ActionValue :type Boolean) (ElapsedSeconds :type Float%20%28double-precision%29) (TriggeredSeconds :type Float%20%28double-precision%29) (InputAction :type Input%20Action%20Object%20Reference :default "/Game/inputs/IA_Menu.IA_Menu"))
  (:Started
    (CallFunction|ToggleMenu)))

(event Input|EnhancedActionEvents|EnhancedInputActionIA_Move
  (params (ActionValue :type Vector%202D%20Structure) (ElapsedSeconds :type Float%20%28double-precision%29) (TriggeredSeconds :type Float%20%28double-precision%29) (InputAction :type Input%20Action%20Object%20Reference :default "/Game/ThirdPerson/Input/Actions/IA_Move.IA_Move"))
  (bind _self self)
  (bind _self_2 self)
  (bind _charactermovement (Variables|Character|GetCharacterMovement _self_2))
  (bind _charactermovement_2 (Variables|Character|GetCharacterMovement _self))
  (bind _returnvalue (Pawn|Components|PawnMovement|GetLastInputVector _charactermovement_2))
  (bind _returnvalue_2 (Math|Vector|VectorLength _returnvalue))
  (if (<= _returnvalue_2 1e+01)
    (Variables|/Script/Engine.CharacterMovementComponent|SetMaxWalkSpeed _charactermovement 1.2e+02)
    (elif (<= _returnvalue_2 15.0)
      (Variables|/Script/Engine.CharacterMovementComponent|SetMaxWalkSpeed _charactermovement 1.8e+02)
      (elif (<= _returnvalue_2 2e+01)
        (Variables|/Script/Engine.CharacterMovementComponent|SetMaxWalkSpeed _charactermovement 2.4e+02)
        (elif (<= _returnvalue_2 25.0)
          (Variables|/Script/Engine.CharacterMovementComponent|SetMaxWalkSpeed _charactermovement 3e+02)
          (elif (<= _returnvalue_2 3e+01)
            (Variables|/Script/Engine.CharacterMovementComponent|SetMaxWalkSpeed _charactermovement 3.6e+02)
            (elif (<= _returnvalue_2 35.0)
              (Variables|/Script/Engine.CharacterMovementComponent|SetMaxWalkSpeed _charactermovement 4.2e+02)
              (elif (<= _returnvalue_2 4e+01)
                (Variables|/Script/Engine.CharacterMovementComponent|SetMaxWalkSpeed _charactermovement 4.8e+02)
                (elif (<= _returnvalue_2 45.0)
                  (Variables|/Script/Engine.CharacterMovementComponent|SetMaxWalkSpeed _charactermovement 5.4e+02)
                  (elif (<= _returnvalue_2 51.0)
                    (Variables|/Script/Engine.CharacterMovementComponent|SetMaxWalkSpeed _charactermovement 6e+02)
                    (else
                      (Development|PrintText (Utilities|Text|ToText(Float) _returnvalue_2 "HalfToEven") true true "(R=1.000000,G=0.015308,B=0.114966,A=1.000000)" 5e+01))))))))))))

(event Input|EnhancedActionEvents|EnhancedInputActionIA_Settings
  (params (ActionValue :type Boolean) (ElapsedSeconds :type Float%20%28double-precision%29) (TriggeredSeconds :type Float%20%28double-precision%29) (InputAction :type Input%20Action%20Object%20Reference :default "/Game/inputs/IA_Settings.IA_Settings"))
  (bind _returnvalue (Game|GetPlayerController 0))
  (bind _returnvalue_2 (UserInterface|CreateWidget "/Game/UI/Inventory/WBP_Options_Menu.WBP_Options_Menu_C"))
  (UserInterface|Viewport|AddtoViewport _returnvalue_2 0)
  (Variables|/Script/Engine.PlayerController|SetbShowMouseCursor _returnvalue true)
  (Input|SetInputModeUIOnly _returnvalue 0 "DoNotLock" false)
  (Game|SetGamePaused true))

(event EventBeginPlay)

(event Collision|EventActorBeginOverlap
  (params (OtherActor :type Actor%20Object%20Reference)))

(event EventTick
  (params (DeltaSeconds :type Float%20%28single-precision%29)))

(fn ConstructionScript)

(fn ToggleMenu
  (bind _returnvalue (Game|GetPlayerController 0))
  (bind _returnvalue_2 (UserInterface|CreateWidget "/Game/UI/Menu/WBP_Menu.WBP_Menu_C"))
  (UserInterface|Viewport|AddtoViewport _returnvalue_2 0)
  (bind _output_get (Variables|Default|SetMenuWidget _returnvalue_2))
  (Variables|Default|SetIsMenuOpen true)
  (Variables|/Script/Engine.PlayerController|SetbShowMouseCursor _returnvalue true)
  (Input|SetInputModeUIOnly _returnvalue _output_get "LockOnCapture" false)
  (Game|SetGamePaused true))